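; Floor actor for an endless runner whose material scrolls faster as the game's difficulty changes.
; The construction script creates a dynamic material instance on the Plane mesh from the floor material.
; BeginPlay caches the EndlessRunner game mode, and each Tick sets the material's ScrollSpeed parameter to StartSpeed scaled by half the current difficulty.
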(event EventBeginPlay
  (bind _asendless_runner_game_mode (Utilities|Casting|CastToEndlessRunnerGameMode (Game|GetGameMode)))
  (Variables|Default|SetAs%20Endless%20Runner%20Game%20Mode _asendless_runner_game_mode))

(event Collision|EventActorBeginOverlap
  (params (OtherActor :type Actor%20Object%20Reference)))

(event EventTick
  (params (DeltaSeconds :type Float%20%28single-precision%29))
  (Rendering|Material|SetScalarParameterValue (Variables|Default|GetFloorMat) "ScrollSpeed" (* (Variables|Default|GetStartSpeed) (/ (Class|EndlessRunnerGameMode|GetDifficulty (Variables|Default|GetAs%20Endless%20Runner%20Game%20Mode)) 2.0)) :!class /Script/Engine.MaterialInstanceDynamic))

(fn ConstructionScript
  (bind _returnvalue (Rendering|Material|CreateDynamicMaterialInstance (Variables|Default|GetPlane) 0 "/Game/Materials/Floor_Inst.Floor_Inst" "None" :!class /Script/Engine.PrimitiveComponent))
  (Variables|Default|SetFloorMat _returnvalue))