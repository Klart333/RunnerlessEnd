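; Tree actor for an endless runner that scrolls along the world X axis.
; On BeginPlay it caches the EndlessRunnerGameMode.
; Each tick it offsets itself without sweep by Speed times the game mode's difficulty, with no delta-time scaling, so movement depends on frame rate.
; It destroys itself once its X position reaches a fixed limit.
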(event EventBeginPlay
  (bind _asendless_runner_game_mode (Utilities|Casting|CastToEndlessRunnerGameMode (Game|GetGameMode)))
  (Variables|Default|SetAs%20Endless%20Runner%20Game%20Mode _asendless_runner_game_mode))

(event Collision|EventActorBeginOverlap
  (params (OtherActor :type Actor%20Object%20Reference)))

(event EventTick
  (params (DeltaSeconds :type Float%20%28single-precision%29))
  (Transformation|AddActorWorldOffset (Math|Vector|MakeVector (* (Variables|Default|GetSpeed) (Class|EndlessRunnerGameMode|GetDifficulty (Variables|Default|GetAs%20Endless%20Runner%20Game%20Mode))) 0.0 0.0))
  (if (>= (.X (Class|KismetMathLibrary|BreakVector3f (Transformation|GetActorLocation))) 1e+03)
    (Actor|DestroyActor)))

(fn ConstructionScript)